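; AI controller that drives its pawn with the Bt_followd behavior tree.
; On BeginPlay it sets up the Bb_ai blackboard, then, if a controlled pawn is valid, saves that pawn's location as HomeLoc and starts the tree.
; GetBAttack combines the Q, W, E and R attack flags into one boolean that is true when any is set.
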(event `self.ReceiveBeginPlay`
  (bind _returnvalue (`self.K2_GetPawn`))
  (`self.UseBlackboard` "/Game/Blueprints/AI/bb_ai.bb_ai")
  (`/Engine/EditorBlueprintResources/StandardMacros.IsValid` _returnvalue
    (:`Is Valid`
      (`BlackboardComponent.SetValueAsVector` (`AIBlueprintHelperLibrary.GetBlackboard` self) (`self.home_loc`) (`self.K2_GetActorLocation` _returnvalue))
      (`self.RunBehaviorTree` "/Game/Blueprints/AI/bt_followd.bt_followd"))))

(fn `get_b_attack`
  (returns (res :type Boolean))
  (return (or (`self.b_attack_q`) (`self.b_attack_w`) (`self.b_attack_e`) (`self.b_attack_r`))))

(fn `UserConstructionScript`)