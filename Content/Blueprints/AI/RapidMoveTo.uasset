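; RapidMoveTo is a Behavior Tree task that moves the AI's controlled pawn toward the actor stored in the TargetToFollow blackboard key.
; On every tick it reissues AIMoveTo with a small fixed acceptance radius, first casting and caching the owning bp_ai_controller if needed.
; A successful move finishes the task as failed, and no other move outcome finishes it.
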(event `self.ReceiveTick`
  (params (OwnerActor :type "Actor Object Reference") (DeltaSeconds :type "Float (single-precision)"))
  ;[1 1 1] 获得Controller
  (if (not (!= (`self.AI_CON_Ref`) null))
    (bind _asbp_ai_controller (cast `/Game/Blueprints/AI/bp_ai_controller` OwnerActor))
    (set `self.AI_CON_Ref` _asbp_ai_controller))
  ;[1 1 1] 真正开始移动
  (`|AIMoveTo` (`Controller.K2_GetPawn` (`self.AI_CON_Ref`)) (0.0 0.0 0.0) (`BTFunctionLibrary.GetBlackboardValueAsActor` (`self.target_to_follow`)) 50.0
    (:`OnSuccess`
      (`self.FinishExecute` false))))