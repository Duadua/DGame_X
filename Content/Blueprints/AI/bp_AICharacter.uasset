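; AI character Blueprint that deals melee-style contact damage and displays a floating health bar.
; When its Box overlaps a non-AICharacter actor while the AI controller's attack flag is set, it sends Attack damage through DamageInterface.
; Each Tick it pushes the health ratio into the blood bar widget and rotates that component to face the player camera.
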(event `self.Box.OnComponentBeginOverlap`
  (params (OverlappedComponent :type "PrimitiveComponent Object Reference") (OtherActor :type "Actor Object Reference") (OtherComp :type "PrimitiveComponent Object Reference") (OtherBodyIndex :type Integer) (bFromSweep :type Boolean) (SweepResult :type "HitResult Structure (by ref)"))
  ;[1 1 1] 攻击时碰撞造成伤害
  (bind _asbp_ai_controller (cast `/Game/Blueprints/AI/bp_ai_controller` (`self.GetController`)))
  (bind _res (`/Game/Blueprints/AI/bp_ai_controller.get_b_attack` _asbp_ai_controller))
  (if _res
    (if (!= (`GameplayStatics.GetObjectClass` OtherActor) "bp_AICharacter_C")
      (if (`KismetSystemLibrary.DoesImplementInterface` OtherActor "/Script/DGame.DamageInterface")
        (message `DamageInterface.DoDamage` OtherActor (`self.attack`))))))

(event `self.ReceiveTick`
  (params (DeltaSeconds :type "Float (single-precision)"))
  (bind _bloodbar (`self.BloodBar`))
  ;[1 1 1] update blood
  (bind _asbp_umg_blood (cast `/Game/Blueprints/UI/bp_umg_blood` (`WidgetComponent.GetUserWidgetObject` (`self.BloodBar`))))
  (`ProgressBar.SetPercent` (`/Game/Blueprints/UI/bp_umg_blood.bar_blood` _asbp_umg_blood) (/ (`self.health`) (`self.health_max`)))
  ;[1 1 1] 始终朝向镜头
  (`SceneComponent.K2_SetWorldRotation` _bloodbar (`KismetMathLibrary.MakeRotFromX` (- (`self.K2_GetActorLocation` (`PlayerController.PlayerCameraManager` (`GameplayStatics.GetPlayerController` 0))) (`SceneComponent.K2_GetComponentLocation` _bloodbar))) false false))

(fn `UserConstructionScript`)