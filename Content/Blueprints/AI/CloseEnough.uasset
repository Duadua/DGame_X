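; Behavior tree decorator that gates AI behavior on the controlled pawn's distance to its follow target.
; It casts the owner to bp_ai_controller, reads the TargetToFollow actor from the blackboard and measures the straight-line distance between target and pawn.
; Despite the name CloseEnough, the check passes when that distance is at or beyond AcceptableDistance.
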(fn `PerformConditionCheck`
  (params (OwnerActor :type "Actor Object Reference"))
  (returns (ReturnValue :type Boolean))
  (bind _asbp_ai_controller (cast `/Game/Blueprints/AI/bp_ai_controller` OwnerActor))
  (set `self.AI_CON_Ref` _asbp_ai_controller)
  (return (>= (`KismetMathLibrary.VSize` (- (`Actor.K2_GetActorLocation` (`BTFunctionLibrary.GetBlackboardValueAsActor` (`self.target_to_follow`))) (`Actor.K2_GetActorLocation` (`Controller.K2_GetPawn` (`self.AI_CON_Ref`))))) (`self.AcceptableDistance`))))