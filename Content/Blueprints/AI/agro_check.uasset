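; Behavior Tree aggro check that finds visible objects around the AI and sets them as follow targets.
; Each tick it sphere-traces around the pawn for configured object types, ignoring all Bp_AICharacter actors, using a cached bp_ai_controller reference.
; A debug-drawn Camera-channel line trace tests each hit for line of sight, writing TargetToFollow and TargetLocation or clearing TargetToFollow.
; The last hit processed wins, and an empty sweep leaves the blackboard unchanged.
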(event `self.ReceiveTick`
  (params (OwnerActor :type "Actor Object Reference") (DeltaSeconds :type "Float (single-precision)"))
  (bind _returnvalue (`Actor.K2_GetActorLocation` (`Controller.K2_GetPawn` (`self.AI_CON_Ref`))))
  ;[1 1 1] 获得controller
  (if (not (!= (`self.AI_CON_Ref`) null))
    (bind _asbp_ai_controller (cast `/Game/Blueprints/AI/bp_ai_controller` OwnerActor))
    (set `self.AI_CON_Ref` _asbp_ai_controller))
  (bind _outactors (`GameplayStatics.GetAllActorsOfClass` "/Game/Blueprints/AI/bp_AICharacter.bp_AICharacter_C"))
  ;[1 1 1] 设置当前位置
  (set `self.MyLocation` _returnvalue)
  ;[1 1 1] 设置圆形碰撞检测范围
  (bind _outhits (`KismetSystemLibrary.SphereTraceMultiForObjects` _returnvalue (+ _returnvalue (0.0 0.0 15.0)) 1500.0 (`self.DesiredObjectTypes`) false _outactors))
  (for _array_element _outhits
    (bind (_bblockinghit _binitialoverlap _time _distance _location _impactpoint _normal _impactnormal _physmat _hitactor) (`GameplayStatics.BreakHitResult` _array_element))
    ;[1 1 1] 对于看到的每一个物体发射射线
    (bind _outhit (`KismetSystemLibrary.LineTraceSingle` (`self.MyLocation`) (`Actor.K2_GetActorLocation` _hitactor) "TraceTypeQuery2" false _outactors "ForDuration"))
    (bind (_bblockinghit_2 _binitialoverlap_2 _time_2 _distance_2 _location_2 _impactpoint_2 _normal_2 _impactnormal_2 _physmat_2 _hitactor_2) (`GameplayStatics.BreakHitResult` _outhit))
    (if (== _hitactor_2 _hitactor)
      ;[1 1 1] 将检测到的物体作为移动目标
      (`BTFunctionLibrary.SetBlackboardValueAsObject` (`self.target_to_follow`) _hitactor_2)
      ;[1 1 1] 同时设置移动目标的位置
      (`BTFunctionLibrary.SetBlackboardValueAsVector` (`self.target_location`) (`Actor.K2_GetActorLocation` _hitactor_2))
      (else
        ;[1 1 1] 没有检测到的话清空数据
        (`BTFunctionLibrary.SetBlackboardValueAsObject` (`self.target_to_follow`))))))