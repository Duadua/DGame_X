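; This Blueprint is an enemy spawner that places AI characters at random points inside its SpawnVolume.
; Its spawn_enemy event counts every Bp_AICharacter in the level and spawns one more only while that total is below EnemyMax.
; Each spawn gets a random point in the volume's scaled extent, a random yaw and the Bt_followd behavior tree.
; Nothing in this graph calls the event.
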(event `spawn_enemy`
  (bind _spawnvolume (`self.SpawnVolume`))
  ;[1 1 1] 区域内随机生成敌人
  (bind _outactors (`GameplayStatics.GetAllActorsOfClass` "/Game/Blueprints/AI/bp_AICharacter.bp_AICharacter_C"))
  (if (< (`KismetArrayLibrary.Array_Length` _outactors) (`self.enemy_max`))
    (`AIBlueprintHelperLibrary.SpawnAIFromClass` "/Game/Blueprints/AI/bp_AICharacter.bp_AICharacter_C" "/Game/Blueprints/AI/bt_followd.bt_followd" (`KismetMathLibrary.RandomPointInBoundingBox` (`SceneComponent.K2_GetComponentLocation` _spawnvolume) (`BoxComponent.GetScaledBoxExtent` _spawnvolume)) (`KismetMathLibrary.MakeRotator` 0.0 0.0 (`KismetMathLibrary.RandomFloatInRange` -180.0 180.0)))))

(fn `UserConstructionScript`)