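; Game mode Blueprint that handles player death and respawn, plus cleanup of dead AI characters.
; Tick polls BDeathEnd on the player and every Bp_AICharacter, destroying AI that have finished dying.
; On player death, the loop over AI destroys each one and, within the same body, respawns the player at the origin.
; Each respawn re-initialises and possesses via MyPlayerController, restores action state and camera pitch, and resets MainUi labels.
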(event `self.ReceiveTick`
  (params (DeltaSeconds :type "Float (single-precision)"))
  (bind _returnvalue (`GameplayStatics.GetPlayerController` 0))
  (`|ExecutionSequence`
    (:`then_0`
      ;[1 1 1] 人物死亡
      (bind _asbp_my_character (cast `/Game/Blueprints/Character/bp_MyCharacter` (`GameplayStatics.GetPlayerCharacter` 0)))
      (if (`BaseCharacter.b_death_end` _asbp_my_character)
        ;[1 1 1] 先销毁敌人
        (bind _outactors (`GameplayStatics.GetAllActorsOfClass` "/Game/Blueprints/AI/bp_AICharacter.bp_AICharacter_C"))
        (for _array_element _outactors
          (`self.K2_DestroyActor` _array_element)
          (`self.K2_DestroyActor` (`GameplayStatics.GetPlayerCharacter` 0))
          (bind _returnvalue_2 (`|SpawnActorFromClass` "/Game/Blueprints/Character/bp_MyCharacter.bp_MyCharacter_C" (`KismetMathLibrary.MakeTransform` (0.0 0.0 0.0)) "Undefined" "OverrideRootScale" null null))
          (bind _asmy_player_controller (cast `MyPlayerController` _returnvalue))
          (`MyPlayerController.init` _asmy_player_controller)
          (`Controller.Possess` _asmy_player_controller _returnvalue_2)
          (set `MyPlayerController.controller_state` "E_ACT" _asmy_player_controller)
          (`MyPlayerController.update_controller_state` _asmy_player_controller)
          (`Controller.SetControlRotation` _returnvalue (`KismetMathLibrary.MakeRotator` 0.0 -45.0))
          (`TextBlock.SetText` (`MainWidget.mode_text` (`self.main_ui`)) "动作模式")
          (`TextBlock.SetText` (`MainWidget.fight_state_text` (`self.main_ui`)) "战"))))
    (:`then_1`
      ;[1 1 1] ai死亡
      (bind _outactors_2 (`GameplayStatics.GetAllActorsOfClass` "/Game/Blueprints/AI/bp_AICharacter.bp_AICharacter_C"))
      (for _array_element_2 _outactors_2
        (if (`BaseCharacter.b_death_end` _array_element_2)
          (`self.K2_DestroyActor` _array_element_2))))))

(fn `UserConstructionScript`)