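; Player character Blueprint that deals damage when its Box collision overlaps another actor during an attack.
; On overlap, it reads the attack flag from MyPlayerController and, while that flag is set, ignores itself and checks the other actor for DamageInterface.
; Valid targets receive a DoDamageMessage call carrying the character's Attack value, so no cast to the victim's class is needed.
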(event `self.Box.OnComponentBeginOverlap`
  (params (OverlappedComponent :type "PrimitiveComponent Object Reference") (OtherActor :type "Actor Object Reference") (OtherComp :type "PrimitiveComponent Object Reference") (OtherBodyIndex :type Integer) (bFromSweep :type Boolean) (SweepResult :type "HitResult Structure (by ref)"))
  ;[1 1 1] 攻击时碰撞造成伤害
  (bind _asmy_player_controller (cast `MyPlayerController` (`self.GetController`)))
  (bind _returnvalue (`MyPlayerController.get_b_attack` _asmy_player_controller))
  (if _returnvalue
    (if (!= OtherActor self)
      (if (`KismetSystemLibrary.DoesImplementInterface` OtherActor "/Script/DGame.DamageInterface")
        (message `DamageInterface.DoDamage` OtherActor (`self.attack`))))))

(fn `UserConstructionScript`)